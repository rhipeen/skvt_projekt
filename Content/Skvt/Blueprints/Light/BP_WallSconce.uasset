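; BP_WallSconce is a wall sconce light Blueprint with adjustable on state and appearance.
; Its construction script applies the IsOn flag to SconceLight's visibility, then sets the light's intensity, color and inner and outer cone angles from Blueprint variables.
; A ToggleOn function takes a TurnOn input but has an empty body.
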(fn ConstructionScript
  (bind _sconcelight (Variables|Default|GetSconceLight))
  (Utilities|FlowControl|Sequence
    (:then_0
      (Rendering|SetVisibility _sconcelight (Variables|Light|GetIsOn) false))
    (:then_1
      (Rendering|Components|Light|SetIntensity _sconcelight (Variables|Light|GetBrightness))
      (Rendering|Components|Light|SetLightColor _sconcelight (Variables|Light|GetColor) true)
      (Rendering|Lighting|SetInnerConeAngle _sconcelight (Variables|Light|GetInner%20Cone%20Angle))
      (Rendering|Lighting|SetOuterConeAngle _sconcelight (Variables|Light|GetOuter%20Cone%20Angle)))))

(fn Toggleon
  (params (TurnOn :type Boolean)))